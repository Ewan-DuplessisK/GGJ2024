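; BP_InGameEvents is a Blueprint that presents scripted in-game events, a lynx jumpscare and an incoming train warning, through UI and sound.
; BeginPlay creates and stores an event widget and a lynx widget without displaying them.
; The LynxJumpscare and Train events add their widget to the viewport and play a 2D sound, with Train first setting the warning text.
; Nothing in this Blueprint calls those events or removes the widgets.
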(event `self.ReceiveBeginPlay`
  (bind _returnvalue (`|CreateWidget` "/Game/ThirdPerson/UI/WBP_EventUI.WBP_EventUI_C"))
  (set `self.Event Widget` _returnvalue)
  (bind _returnvalue_2 (`|CreateWidget` "/Game/ThirdPerson/UI/WBP_LynxUI.WBP_LynxUI_C"))
  (set `self.Lynx Widget` _returnvalue_2))

(event `Lynx Jumpscare`
  (`UserWidget.AddToViewport` (`self.Lynx Widget`) 0)
  (`GameplayStatics.PlaySound2D` "/Game/Sounds/Lynx_SFX.Lynx_SFX" 1.0 1.0 0.0 null null))

(event `Train`
  (bind _event_widget (`self.Event Widget`))
  (`/Game/ThirdPerson/UI/WBP_EventUI.Change Event Text` _event_widget "Train Incoming")
  (`UserWidget.AddToViewport` _event_widget 0)
  (`GameplayStatics.PlaySound2D` "/Game/Sounds/Train.Train" 1.0 1.0 0.0 null null))

(fn `UserConstructionScript`)