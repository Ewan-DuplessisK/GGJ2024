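; BP_Train is a train actor that rides the spline of the BP_TrainTrack found in the level and knocks away overlapping player characters.
; Each tick it advances front and back wheel distances by Speed, places both wheel assemblies on the spline and spins the wheels.
; The body sits at their midpoint facing the front one.
; Distances wrap at the spline end, where the train stops unless IsLoop is set.
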(event `self.ReceiveBeginPlay`
  (`self.SplineDetect`
    (:`Out`
      (`self.Detect Wheel Loc`
        (:`Out`
          (set `self.IsStart?` true))))))

(event `self.ReceiveTick`
  (params (DeltaSeconds :type "Float (single-precision)"))
  (set `self.Delta Seconds` DeltaSeconds)
  (if (`self.IsStart?`)
    (`self.SpeedDistance`
      (:`Out`
        (`self.Wheel Start Move`
          (:`Out`
            (`self.Wheel Rotation`
              (:`Out`
                (`self.Move Train`
                  (:`Out`
                    (`|ExecutionSequence`
                      (:`then_0`
                        (bind _distanceout (`self.Loop` (`self.Front Wheel Distance`))
                          (:`Out`
                            (set `self.Front Wheel Distance` _distanceout))))
                      (:`then_1`
                        (bind _distanceout_2 (`self.Loop` (`self.Back Wheel Distance`))
                          (:`Out`
                            (set `self.Back Wheel Distance` _distanceout_2)))))))))))))))

(event `self.Box.OnComponentBeginOverlap`
  (params (OverlappedComponent :type "PrimitiveComponent Object Reference") (OtherActor :type "Actor Object Reference") (OtherComp :type "PrimitiveComponent Object Reference") (OtherBodyIndex :type Integer) (bFromSweep :type Boolean) (SweepResult :type "HitResult Structure (by ref)"))
  (bind (_asbp_game_character _bsuccess) (cast `/Game/ThirdPerson/Blueprints/BP_GameCharacter` OtherActor :!pure true))
  (if _bsuccess
    (`Character.LaunchCharacter` _asbp_game_character (* (`KismetMathLibrary.GetDirectionUnitVector` (`self.K2_GetActorLocation` OtherActor) (`self.K2_GetActorLocation`)) (* (`self.Speed`) -0.7)) false false)))

(fn `UserConstructionScript`)